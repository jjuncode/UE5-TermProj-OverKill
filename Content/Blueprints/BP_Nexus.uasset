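; BP_Nexus is a damageable objective that stores its health in the color of its water material.
; BeginPlay creates dynamic materials for the water and angel parts of the mesh.
; GetDamaged shifts the water toward red by draining blue, then green, tints the angel red, and prints a loss message once the color passes pure red.
; SetAngelColor triggers a delayed reset to white, which calls SetAngelColor again and keeps repeating.
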(event Custom|Set%20Origin%20Color
  (Utilities|FlowControl|Delay 0.2)
  (CallFunction|SetAngelColor "(R=1.000000,G=1.000000,B=1.000000,A=1.000000)"))

(event EventBeginPlay
  (bind _staticmesh (Variables|Default|GetStaticMesh))
  (Utilities|FlowControl|Sequence
    (:then_0
      (bind _returnvalue (Rendering|Material|CreateDynamicMaterialInstance _staticmesh 3 (Class|PrimitiveComponent|GetMaterialbyName _staticmesh "Red") "None" :!class /Script/Engine.PrimitiveComponent))
      (Variables|Default|SetDMI%20Water _returnvalue))
    (:then_1
      (bind _returnvalue_2 (Rendering|Material|CreateDynamicMaterialInstance _staticmesh 1 (Class|PrimitiveComponent|GetMaterialbyName _staticmesh "Angel") "None" :!class /Script/Engine.PrimitiveComponent))
      (bind _output_get (Variables|Default|SetDMI%20Angel _returnvalue_2))
      (Rendering|Material|SetTextureParameterValue _output_get "Color" "/Game/Fab/Blood_Temple/bloodtemplefbx/Textures/bloodtemplefbx_texture_5.bloodtemplefbx_texture_5"))))

(event Collision|EventActorBeginOverlap
  (params (OtherActor :type Actor%20Object%20Reference)))

(fn ConstructionScript)

(fn GetDamaged
  (bind _damagevalue (LocalVariables|GetDamageValue))
  (bind _dmi_water (Variables|Default|GetDMI%20Water))
  (bind _returnvalue (* _damagevalue -1.0))
  (Development|PrintText "Damaged")
  (bind _returnvalue_2 (Rendering|Material|GetVectorParameterValue _dmi_water "Color" :!class /Script/Engine.MaterialInstanceDynamic))
  (Utilities|FlowControl|Sequence
    (:then_0
      ;[0.15 0.15 0.15 0.5] Dynamic Material - Water Life Color Change
      (if (> (.b _returnvalue_2) 0.0)
        (Rendering|Material|SetVectorParameterValue _dmi_water "Color" (- (Utilities|Struct|MakeLinearColor (.r _returnvalue_2) (.g _returnvalue_2) (.b _returnvalue_2) 1.0) (Utilities|Struct|MakeLinearColor _returnvalue 0.0 _damagevalue 0.0)) :!class /Script/Engine.MaterialInstanceDynamic)
        (else
          (Rendering|Material|SetVectorParameterValue _dmi_water "Color" (- (Utilities|Struct|MakeLinearColor (.r _returnvalue_2) (.g _returnvalue_2) (.b _returnvalue_2) 1.0) (Utilities|Struct|MakeLinearColor _returnvalue _damagevalue 0.0 0.0)) :!class /Script/Engine.MaterialInstanceDynamic))))
    (:then_1
      (CallFunction|SetAngelColor "(R=1.000000,G=0.000000,B=0.000000,A=1.000000)"))
    (:then_2
      ;[0.15 0.15 0.15 0.5] You Lose
      (if (Math|Boolean|ANDBoolean (> (.r _returnvalue_2) 1.0) (< (.g _returnvalue_2) 0.0) (< (.b _returnvalue_2) 0.0))
        (Development|PrintText "You Lose!")))))

(fn SetAngelColor
  (params (Color :type Linear%20Color%20Structure))
  (Rendering|Material|SetVectorParameterValue (Variables|Default|GetDMI%20Angel) "Color" Color :!class /Script/Engine.MaterialInstanceDynamic)
  (CallFunction|SetOriginColor))