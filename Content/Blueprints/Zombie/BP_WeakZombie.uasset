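; BP_WeakZombie is a zombie enemy that walks straight at the BP_Nexus and attacks it.
; Each tick it steers along the flat direction to the Nexus, or within range plays alternating attack montages whose "Attack" notify damages the Nexus.
; A Nexus event binding boosts its walk speed up to a cap.
; A single GetDamaged call marks it dead, stopping that logic and disabling capsule collision.
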(event Custom|Strengthen
  (bind _charactermovement (Variables|Character|GetCharacterMovement))
  ;[0.15 0.15 0.15 0.5] Bind Event
  ;[0.15 0.15 0.15 0.5] Strengthen
  (Variables|/Script/Engine.CharacterMovementComponent|SetMaxWalkSpeed _charactermovement (Math|Float|Min(Float) (* (Class|MovementComponent|GetMaxSpeed _charactermovement) 1.5) 267.0)))

(event EventBeginPlay
  (bind _charactermovement (Variables|Character|GetCharacterMovement))
  (Utilities|FlowControl|Sequence
    (:then_0
      ;[0.15 0.15 0.15 0.5] Caching
      (bind _returnvalue (Actor|GetActorOfClass "/Game/Blueprints/Revenant/BP_Revenant.BP_Revenant_C"))
      (Variables|Default|SetRevenant _returnvalue)
      (bind _returnvalue_2 (Actor|GetActorOfClass "/Game/Blueprints/BP_Nexus.BP_Nexus_C"))
      (Variables|Default|SetNexus _returnvalue_2)
      ;[0.15 0.15 0.15 0.5] Bind Event
      (EventDispatchers|BindEventtoStrengthenZombie (Variables|Default|GetNexus) (delegate Custom|Strengthen)))
    (:then_1
      ;[0.15 0.15 0.15 0.5] Set Speed
      (Variables|/Script/Engine.CharacterMovementComponent|SetMaxWalkSpeed _charactermovement (Variables|Default|GetSpawnSpeed))
      (Variables|/Script/Engine.CharacterMovementComponent|SetMaxAcceleration _charactermovement 2e+03))))

(event EventGetDamaged
  (Variables|Default|SetDeath true)
  (Collision|SetCollisionEnabled (Variables|Collision|GetCapsuleComponent) "NoCollision"))

(event EventTick
  (params (DeltaSeconds :type Float%20%28single-precision%29))
  (bind _returnvalue (Transformation|GetActorLocation))
  (bind _nexus (Variables|Default|GetNexus))
  (bind _returnvalue_2 (Transformation|GetActorLocation _nexus))
  (bind _returnvalue_3 (- _returnvalue_2 _returnvalue))
  ;[0.15 0.15 0.15 0.5] Get Target Distn
  (Variables|Default|SetSpeed (Math|Vector|VectorLengthXY (Transformation|GetVelocity)))
  (if (not (Variables|Default|GetDeath))
    (Variables|Default|SetTargetDistn (Math|Vector|MakeVector (.x _returnvalue_3) (.y _returnvalue_3) 0.0))
    ;[0.15 0.15 0.15 0.5] Attack
    (if (< (Math|Vector|VectorLength (Variables|Default|GetTargetDistn)) 1.3e+02)
      (Utilities|FlowControl|DoOnce false :!label _label
        (:Completed
          (Utilities|FlowControl|FlipFlop
            (:A
              (bind _notifyname (Animation|Montage|PlayMontage (Variables|Character|GetMesh) "/Game/Asset/Zombie/Animation/AM_ZombieAttack.AM_ZombieAttack" 1.0 0.0 "Attack1")
                (:OnCompleted
                  (goto _label Reset))
                (:OnNotifyBegin
                  (if (== _notifyname "Attack")
                    (Default|GetDamaged (Variables|Default|GetNexus) :!label _label_2)))))
            (:B
              (bind _notifyname_2 (Animation|Montage|PlayMontage (Variables|Character|GetMesh) "/Game/Asset/Zombie/Animation/AM_ZombieAttack.AM_ZombieAttack" 1.0 0.0 "Attack2")
                (:OnCompleted
                  (goto _label Reset))
                (:OnNotifyBegin
                  (if (== _notifyname_2 "Attack")
                    (goto _label_2))))))))
      (else
        ;[0.15 0.15 0.15 0.5] Move Toward to Target
        (Pawn|Input|AddMovementInput (Math|Vector|Normalize (Variables|Default|GetTargetDistn)) 1.0 false)
        (Transformation|SetActorRotation (Math|Conversions|RotationFromXVector (Math|Vector|Normalize (Variables|Default|GetTargetDistn))))))))

(fn ConstructionScript)