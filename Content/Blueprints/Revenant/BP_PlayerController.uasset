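; Player controller for BP_Revenant that handles move and look, manages the HUD widgets and runs an execution quick-time event.
; Tick feeds ammo and execution stacks to the HUD and toggles the crosshair by pawn state.
; CreateInputAction removes the IMC_Soldier mapping context and shows seven random WASD prompts.
; Correct in-order presses hide prompts and trigger ExecuteAction; clearing all calls ExecuteDone and restores input after a short delay.
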(event Input|EnhancedActionEvents|EnhancedInputActionIA_Turn
  (params (ActionValue :type Vector%202D%20Structure) (ElapsedSeconds :type Float%20%28double-precision%29) (TriggeredSeconds :type Float%20%28double-precision%29) (InputAction :type Input%20Action%20Object%20Reference :default "/Game/Asset/Input/IA_Turn.IA_Turn"))
  ;[0.15 0.15 0.15 0.5] Turn
  (Class|PlayerController|AddYawInput (.x ActionValue))
  (Class|PlayerController|AddPitchInput (.y ActionValue)))

(event Input|EnhancedActionEvents|EnhancedInputActionIA_Move
  (params (ActionValue :type Vector%202D%20Structure) (ElapsedSeconds :type Float%20%28double-precision%29) (TriggeredSeconds :type Float%20%28double-precision%29) (InputAction :type Input%20Action%20Object%20Reference :default "/Game/Asset/Input/IA_Move.IA_Move"))
  (bind _returnvalue (Pawn|GetControlRotation :!class /Script/Engine.Controller))
  (bind _rvenant (Variables|Default|GetRvenant))
  ;[0.15 0.15 0.15 0.5] RPG Move
  (Pawn|Input|AddMovementInput _rvenant (Math|Vector|GetForwardVector (Math|Rotator|MakeRotator 0.0 0.0 (.yaw _returnvalue))) (.x ActionValue) false)
  (Pawn|Input|AddMovementInput _rvenant (Math|Vector|GetRightVector (Math|Rotator|MakeRotator 0.0 0.0 (.yaw _returnvalue))) (.y ActionValue) false))

(event EventBeginPlay
  (CallFunction|EnableInput)
  (bind _asbp_revenant (Utilities|Casting|CastToBP_Revenant (Pawn|GetControlledPawn)))
  (Variables|Default|SetRvenant _asbp_revenant)
  (bind _returnvalue (UserInterface|CreateWidget "/Game/Blueprints/WBP_Ammo.WBP_Ammo_C"))
  (bind _output_get (Variables|Default|SetAmmoWidget _returnvalue))
  (UserInterface|Viewport|AddtoViewport _output_get 0)
  (bind _returnvalue_2 (UserInterface|CreateWidget "/Game/Blueprints/WBP_InputAction.WBP_InputAction_C"))
  (bind _output_get_2 (Variables|Default|SetInputActionWidget _returnvalue_2))
  (UserInterface|Viewport|AddtoViewport _output_get_2 0)
  (Variables|/Script/UMG.Widget|SetVisibility _output_get_2 "Hidden")
  (bind _returnvalue_3 (UserInterface|CreateWidget "/Game/Blueprints/WBP_CrossHair.WBP_CrossHair_C"))
  (bind _output_get_3 (Variables|Default|SetCrossHairWidget _returnvalue_3))
  (UserInterface|Viewport|AddtoViewport _output_get_3 0))

(event EventTick
  (params (DeltaSeconds :type Float%20%28single-precision%29))
  (bind _rvenant (Variables|Default|GetRvenant))
  (bind _crosshairwidget (Variables|Default|GetCrossHairWidget))
  (bind _ammowidget (Variables|Default|GetAmmoWidget))
  ;[0.15 0.15 0.15 0.5] Ammo UI
  (Class|BPIHUD|GetAmmo(Message) _ammowidget (Variables|/Game/Blueprints/Revenant/BP_Revenant.BP_Revenant_C|GetAmmo _rvenant))
  (Default|SetExecutionStack _ammowidget (Variables|/Game/Blueprints/Revenant/BP_Revenant.BP_Revenant_C|GetExecutionStack _rvenant))
  ;[0.15 0.15 0.15 0.5] Cross Hair Visibility
  (if (Utilities|Enum|Equal(Enum) (Variables|/Game/Blueprints/Revenant/BP_Revenant.BP_Revenant_C|GetState (Variables|Default|GetRvenant)) "NewEnumerator0")
    (Widget|SetVisibility _crosshairwidget "Visible")
    (else
      (Widget|SetVisibility _crosshairwidget "Hidden"))))

(event Input|KeyboardEvents|D
  (params (Key :type Key%20Structure :default "None"))
  ;[0.15 0.15 0.15 0.5] Execution Pattern
  (:Pressed
    (Utilities|FlowControl|DoOnce false :!label _label
      (:Completed
        (if (Variables|Default|GetIsExecuting)
          (bind _output_get (Variables|Default|SetKey (Class|KismetInputLibrary|KeyGetDisplayName Key true)))
          (bind _isequal (CallFunction|ProcessEqualInputAction _output_get))
          (if _isequal
            (Default|ExecuteAction (Variables|Default|GetRvenant))
            (if (== (Utilities|Array|Length (Variables|Default|GetInputActionText)) 0)
              (Utilities|FlowControl|Delay 0.3)
              (Variables|Default|SetIsExecuting false)
              (Default|ExecuteDone (Variables|Default|GetRvenant))
              (CallFunction|EnableInput)))))))
  (:Released
    (goto _label Reset)))

(event Input|KeyboardEvents|W
  (params (Key :type Key%20Structure :default "None"))
  ;[0.15 0.15 0.15 0.5] Execution Pattern
  (:Pressed
    (Utilities|FlowControl|DoOnce false :!label _label
      (:Completed
        (if (Variables|Default|GetIsExecuting)
          (bind _output_get (Variables|Default|SetKey (Class|KismetInputLibrary|KeyGetDisplayName Key true)))
          (bind _isequal (CallFunction|ProcessEqualInputAction _output_get))
          (if _isequal
            (Default|ExecuteAction (Variables|Default|GetRvenant))
            (if (== (Utilities|Array|Length (Variables|Default|GetInputActionText)) 0)
              (Utilities|FlowControl|Delay 0.3)
              (Variables|Default|SetIsExecuting false)
              (Default|ExecuteDone (Variables|Default|GetRvenant))
              (CallFunction|EnableInput)))))))
  (:Released
    (goto _label Reset)))

(event Input|KeyboardEvents|S
  (params (Key :type Key%20Structure :default "None"))
  ;[0.15 0.15 0.15 0.5] Execution Pattern
  (:Pressed
    (Utilities|FlowControl|DoOnce false :!label _label
      (:Completed
        (if (Variables|Default|GetIsExecuting)
          (bind _output_get (Variables|Default|SetKey (Class|KismetInputLibrary|KeyGetDisplayName Key true)))
          (bind _isequal (CallFunction|ProcessEqualInputAction _output_get))
          (if _isequal
            (Default|ExecuteAction (Variables|Default|GetRvenant))
            (if (== (Utilities|Array|Length (Variables|Default|GetInputActionText)) 0)
              (Utilities|FlowControl|Delay 0.3)
              (Variables|Default|SetIsExecuting false)
              (Default|ExecuteDone (Variables|Default|GetRvenant))
              (CallFunction|EnableInput)))))))
  (:Released
    (goto _label Reset)))

(event Input|KeyboardEvents|A
  (params (Key :type Key%20Structure :default "None"))
  ;[0.15 0.15 0.15 0.5] Execution Pattern
  (:Pressed
    (Utilities|FlowControl|DoOnce false :!label _label
      (:Completed
        (if (Variables|Default|GetIsExecuting)
          (bind _output_get (Variables|Default|SetKey (Class|KismetInputLibrary|KeyGetDisplayName Key true)))
          (bind _isequal (CallFunction|ProcessEqualInputAction _output_get))
          (if _isequal
            (Default|ExecuteAction (Variables|Default|GetRvenant))
            (if (== (Utilities|Array|Length (Variables|Default|GetInputActionText)) 0)
              (Utilities|FlowControl|Delay 0.3)
              (Variables|Default|SetIsExecuting false)
              (Default|ExecuteDone (Variables|Default|GetRvenant))
              (CallFunction|EnableInput)))))))
  (:Released
    (goto _label Reset)))

(fn ConstructionScript)

(fn CreateInputAction
  (bind _inputactionwidget (Variables|Default|GetInputActionWidget))
  (bind _inputactionwidget_2 (Variables|Default|GetInputActionWidget))
  (Variables|Default|SetIsExecuting true)
  (CallFunction|DisableInput)
  (Utilities|FlowControl|Sequence
    (:then_0
      (Variables|/Game/Blueprints/WBP_InputAction.WBP_InputAction_C|SetCanVisible_0 _inputactionwidget_2 true))
    (:then_1
      (Variables|/Game/Blueprints/WBP_InputAction.WBP_InputAction_C|SetCanVisible_1 _inputactionwidget_2 true))
    (:then_2
      (Variables|/Game/Blueprints/WBP_InputAction.WBP_InputAction_C|SetCanVisible_2 _inputactionwidget_2 true))
    (:then_3
      (Variables|/Game/Blueprints/WBP_InputAction.WBP_InputAction_C|SetCanVisible_3 _inputactionwidget_2 true))
    (:then_4
      (Variables|/Game/Blueprints/WBP_InputAction.WBP_InputAction_C|SetCanVisible_4 _inputactionwidget_2 true))
    (:then_5
      (Variables|/Game/Blueprints/WBP_InputAction.WBP_InputAction_C|SetCanVisible_5 _inputactionwidget_2 true))
    (:then_6
      (Variables|/Game/Blueprints/WBP_InputAction.WBP_InputAction_C|SetCanVisible_6 _inputactionwidget_2 true)
      (Variables|/Script/UMG.Widget|SetVisibility (Variables|Default|GetInputActionWidget) "Visible")
      (for _index (range 0 6)
        (switch int _index
          (:0
            (bind _newparam (CallFunction|GetRandomChar))
            (Variables|/Game/Blueprints/WBP_InputAction.WBP_InputAction_C|SetInputActionText_0 _inputactionwidget _newparam))
          (:1
            (bind _newparam_2 (CallFunction|GetRandomChar))
            (Variables|/Game/Blueprints/WBP_InputAction.WBP_InputAction_C|SetInputActionText_1 _inputactionwidget _newparam_2))
          (:2
            (bind _newparam_3 (CallFunction|GetRandomChar))
            (Variables|/Game/Blueprints/WBP_InputAction.WBP_InputAction_C|SetInputActionText_2 _inputactionwidget _newparam_3))
          (:3
            (bind _newparam_4 (CallFunction|GetRandomChar))
            (Variables|/Game/Blueprints/WBP_InputAction.WBP_InputAction_C|SetInputActionText_3 _inputactionwidget _newparam_4))
          (:4
            (bind _newparam_5 (CallFunction|GetRandomChar))
            (Variables|/Game/Blueprints/WBP_InputAction.WBP_InputAction_C|SetInputActionText_4 _inputactionwidget _newparam_5))
          (:5
            (bind _newparam_6 (CallFunction|GetRandomChar))
            (Variables|/Game/Blueprints/WBP_InputAction.WBP_InputAction_C|SetInputActionText_5 _inputactionwidget _newparam_6))
          (:6
            (bind _newparam_7 (CallFunction|GetRandomChar))
            (Variables|/Game/Blueprints/WBP_InputAction.WBP_InputAction_C|SetInputActionText_6 _inputactionwidget _newparam_7)))))))

(fn GetRandomChar
  (bind _inputactiontext (Variables|Default|GetInputActionText))
  (switch int (Math|Random|RandomIntegerinRange 1 4)
    (:1
      (bind _output_get (LocalVariables|SetNewLocalVar "W"))
      (Utilities|Array|Add _inputactiontext _output_get))
    (:2
      (bind _output_get_2 (LocalVariables|SetNewLocalVar "S"))
      (Utilities|Array|Add _inputactiontext _output_get_2))
    (:3
      (bind _output_get_3 (LocalVariables|SetNewLocalVar "A"))
      (Utilities|Array|Add _inputactiontext _output_get_3))
    (:4
      (bind _output_get_4 (LocalVariables|SetNewLocalVar "D"))
      (Utilities|Array|Add _inputactiontext _output_get_4)))
  (return (LocalVariables|GetNewLocalVar)))

(fn DisableInput
  (Input|RemoveMappingContext (PlayerController|LocalPlayerSubsystems|GetEnhancedInputLocalPlayerSubsystem) "/Game/Asset/Input/IMC_Soldier.IMC_Soldier" "(bIgnoreAllPressedKeysUntilRelease=True,bForceImmediately=False,bNotifyUserSettings=False)"))

(fn EnableInput
  (Input|AddMappingContext (PlayerController|LocalPlayerSubsystems|GetEnhancedInputLocalPlayerSubsystem) "/Game/Asset/Input/IMC_Soldier.IMC_Soldier" 0 "(bIgnoreAllPressedKeysUntilRelease=True,bForceImmediately=False,bNotifyUserSettings=False)"))

(fn ProcessEqualInputAction
  (params (B :type Text%20%28by%20ref%29))
  (bind _inputactiontext (Variables|Default|GetInputActionText))
  (bind _inputactionwidget (Variables|Default|GetInputActionWidget))
  (bind _output_get (LocalVariables|SetNewLocalVar_0 (Utilities|Enum|Equal(Enum) (Utilities|Array|Get(acopy) (Variables|Default|GetInputActionText)) B)))
  (if _output_get
    (switch int (- 7 (Utilities|Array|Length _inputactiontext))
      (:0
        (Variables|/Game/Blueprints/WBP_InputAction.WBP_InputAction_C|SetCanVisible_0 _inputactionwidget false))
      (:1
        (Variables|/Game/Blueprints/WBP_InputAction.WBP_InputAction_C|SetCanVisible_1 _inputactionwidget false))
      (:2
        (Variables|/Game/Blueprints/WBP_InputAction.WBP_InputAction_C|SetCanVisible_2 _inputactionwidget false))
      (:3
        (Variables|/Game/Blueprints/WBP_InputAction.WBP_InputAction_C|SetCanVisible_3 _inputactionwidget false))
      (:4
        (Variables|/Game/Blueprints/WBP_InputAction.WBP_InputAction_C|SetCanVisible_4 _inputactionwidget false))
      (:5
        (Variables|/Game/Blueprints/WBP_InputAction.WBP_InputAction_C|SetCanVisible_5 _inputactionwidget false))
      (:6
        (Variables|/Game/Blueprints/WBP_InputAction.WBP_InputAction_C|SetCanVisible_6 _inputactionwidget false)))
    (Utilities|Array|RemoveIndex _inputactiontext))
  (return (LocalVariables|GetNewLocalVar_0)))

(fn SetCrossHairPosition
  (params (x :type Float%20%28double-precision%29) (y :type Float%20%28double-precision%29))
  (Class|UserWidget|SetPositioninViewport (Variables|Default|GetCrossHairWidget) (Math|Vector2D|MakeVector2D x y) true))